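; Base Blueprint for interactable objects that register themselves as the player's current interactable while PlayerBP is inside their trigger area.
; Begin and end overlap set and clear that reference, and BeginPlay catches a player already inside.
; EnterThisInteractable forwards non-enterable objects to InteractWithThis, which is an empty hook like ExitThisInteractable.
; The construction script positions the trigger, enter point and mesh from transform variables.
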(event OnComponentBeginOverlap(InteractableArea)
  (params (OverlappedComponent :type Primitive%20Component%20Object%20Reference) (OtherActor :type Actor%20Object%20Reference) (OtherComp :type Primitive%20Component%20Object%20Reference) (OtherBodyIndex :type Integer) (bFromSweep :type Boolean) (SweepResult :type Hit%20Result%20Structure%20%28by%20ref%29))
  (bind _asplayer_bp (Utilities|Casting|CastToPlayerBP OtherActor))
  (Variables|/Game/Blueprints/PlayerBP.PlayerBP_C|SetCurrentInteractable _asplayer_bp self)
  (Variables|Default|SetInArea? true)
  (Variables|Default|SetThePlayer _asplayer_bp))

(event OnComponentEndOverlap(InteractableArea)
  (params (OverlappedComponent :type Primitive%20Component%20Object%20Reference) (OtherActor :type Actor%20Object%20Reference) (OtherComp :type Primitive%20Component%20Object%20Reference) (OtherBodyIndex :type Integer))
  (bind _asplayer_bp (Utilities|Casting|CastToPlayerBP OtherActor))
  (Variables|/Game/Blueprints/PlayerBP.PlayerBP_C|SetCurrentInteractable _asplayer_bp 0)
  (Variables|Default|SetInArea? false)
  (Variables|Default|SetThePlayer 0))

(event Custom|InteractWithThis)

(event Custom|EnterThisInteractable
  (if (not (Variables|Default|GetEnterable?))
    (CallFunction|InteractwithThis)))

(event Custom|ExitThisInteractable)

(event EventBeginPlay
  (bind _interactablearea (Variables|Default|GetInteractableArea))
  (bind _overlappingactors (Collision|GetOverlappingActors _interactablearea "/Game/Blueprints/PlayerBP.PlayerBP_C" :!class /Script/Engine.PrimitiveComponent))
  (if (> (Utilities|Array|Length _overlappingactors) 0)
    (bind _asplayer_bp (Utilities|Casting|CastToPlayerBP (Utilities|Array|Get(acopy) _overlappingactors)))
    (Variables|/Game/Blueprints/PlayerBP.PlayerBP_C|SetCurrentInteractable _asplayer_bp self)
    (Variables|Default|SetInArea? true)
    (Variables|Default|SetThePlayer _asplayer_bp)))

(event Collision|EventActorBeginOverlap
  (params (OtherActor :type Actor%20Object%20Reference)))

(event EventTick
  (params (DeltaSeconds :type Float%20%28single-precision%29)))

(fn ConstructionScript
  (Utilities|FlowControl|Sequence
    (:then_0
      (Transformation|SetRelativeTransform (Variables|Default|GetInteractableArea) (Variables|Default|GetTriggerTransform) false false))
    (:then_1
      (Transformation|SetRelativeTransform (Variables|Default|GetEnterAtPoint) (Variables|Default|GetEnterAtPointTransform) false false))
    (:then_2
      (Transformation|SetRelativeTransform (Variables|Default|GetStaticMesh) (Variables|Default|GetMeshTransform) false false))))