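; Player controller that acts as the player's dialogue participant and toggles the HUD widget's cursor.
; StartDialogue stores a context between itself and another participant, which SelectDialogueOption advances and clears when dialogue ends.
; After a choice, nodes spoken by the player have their text forwarded through PlayerBP to the radio station Blueprint.
; Participant interface functions are default-returning stubs, except the participant name getter.
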(event EventBeginPlay)

(event EventTick
  (params (DeltaSeconds :type Float%20%28single-precision%29)))

(fn ConstructionScript)

(fn ToggleMyHUDCursor
  (params (Show? :type Boolean))
  (bind _asplayer_hud (Utilities|Casting|CastToPlayerHUD (HUD|GetHUD)))
  (Default|ToggleHUDPointer (Variables|/Game/Widgets/PlayerHUD.PlayerHUD_C|GetTheHUDWidget _asplayer_hud) Show?))

(fn SelectDialogueOption
  (params (Index :type Integer))
  (Utilities|IsValid (Variables|Default|GetActiveContext)
    (:Is%20Valid
      (if (Math|Integer|InRange(Integer) 0 0 (Class|DlgContext|GetOptionNum (Variables|Default|GetActiveContext)) true false)
        (bind _returnvalue (Class|DlgContext|ChooseChild (Variables|Default|GetActiveContext) Index))
        (if (Utilities|Name|Equal(Name) (Class|DlgContext|GetActiveParticipantName (Variables|Default|GetActiveContext)) (Variables|Default|GetMyParticipantName))
          (CallFunction|SetDialogueReplyString (Utilities|String|ToString(Text) (Class|DlgContext|GetActiveNodeText (Variables|Default|GetActiveContext)))))
        (if (not _returnvalue)
          ;[1 1 1] Dialogue has ended. Please reset.
          (Variables|Default|SetActiveContext 0))))))

(fn StartDialogue
  (params (Dialogue :type Dlg%20Dialogue%20Object%20Reference) (OtherParticipant :type Object%20Object%20Reference))
  (bind _returnvalue (Class|DlgManager|StartDialogue2 Dialogue OtherParticipant self))
  (Variables|Default|SetActiveContext _returnvalue))

(fn SetDialogueReplyString
  (params (DialogueReply :type String))
  (bind _asplayer_bp (Utilities|Casting|CastToPlayerBP (Game|GetPlayerCharacter 0)))
  (Default|SendDialogueReplyStringtoRadioStationBP _asplayer_bp DialogueReply))

(fn CheckCondition
  (params (ConditionName :type Name%20%28by%20ref%29 :default "None"))
  (return false))

(fn GetBoolValue
  (params (ValueName :type Name%20%28by%20ref%29 :default "None"))
  (return false))

(fn GetFloatValue
  (params (ValueName :type Name%20%28by%20ref%29 :default "None"))
  (return 0.0))

(fn GetIntValue
  (params (ValueName :type Name%20%28by%20ref%29 :default "None"))
  (return 0))

(fn GetNameValue
  (params (ValueName :type Name%20%28by%20ref%29 :default "None"))
  (return "None"))

(fn GetParticipantDisplayName
  (params (ActiveSpeaker :type Name :default "None"))
  (return ""))

(fn GetParticipantGender
  (return "Masculine"))

(fn GetParticipantIcon
  (params (ActiveSpeaker :type Name :default "None") (ActiveSpeakerState :type Name :default "None"))
  (return 0))

(fn GetParticipantName
  (return (Variables|Default|GetMyParticipantName)))

(fn ModifyBoolValue
  (params (ValueName :type Name%20%28by%20ref%29 :default "None") (bNewValue :type Boolean))
  (return false))

(fn ModifyFloatValue
  (params (ValueName :type Name%20%28by%20ref%29 :default "None") (bDelta :type Boolean) (Value :type Float%20%28single-precision%29))
  (return false))

(fn ModifyIntValue
  (params (ValueName :type Name%20%28by%20ref%29 :default "None") (bDelta :type Boolean) (Value :type Integer))
  (return false))

(fn ModifyNameValue
  (params (ValueName :type Name%20%28by%20ref%29 :default "None") (NameValue :type Name%20%28by%20ref%29 :default "None"))
  (return false))

(fn OnDialogueEvent
  (params (EventName :type Name%20%28by%20ref%29 :default "None"))
  (return false))