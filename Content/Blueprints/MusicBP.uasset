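; Music player actor that plays, pauses and resumes a music track with a toggleable high-pass filter.
; The construction script assigns the track to the audio component, and PauseMusic flip-flops its paused state.
; ToggleFilter alternately plays and reverses a timeline that sweeps the source effect preset's cutoff between minimum and maximum frequencies.
; A gate blocks further filter toggles until each sweep finishes.
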(event Custom|PauseMusic
  (bind _isa (Utilities|FlowControl|FlipFlop)
    (:A
      _)
    (:B
      _))
  (Class|AudioComponent|SetPaused (Variables|Default|GetAudio) _isa))

(event Custom|PlayMusic
  (Audio|Components|Audio|Play (Variables|Default|GetAudio) 0.0))

(event Custom|ToggleFilter
  (Utilities|FlowControl|Gate false :!label _label
    (:Exit
      (Utilities|FlowControl|Sequence
        (:then_0
          (Utilities|FlowControl|FlipFlop
            (:A
              (bind _alpha (Timeline|HighPassTimeline PlayFromStart)
                (:Update
                  (Class|SourceEffectFilterPreset|SetSettings (Variables|Default|GetEffectPreset) (Utilities|Struct|MakeSourceEffectFilterSettings "StateVariable" "HighPass" (Math|Float|Lerp (Variables|Default|GetHighPassMinFrequency) (Variables|Default|GetHighPassMaxFrequency) _alpha) 2.0)))
                (:Finished
                  (goto _label Open))))
            (:B
              (Timeline|HighPassTimeline ReverseFromEnd))))
        (:then_1
          (goto _label Close))))))

(event EventBeginPlay)

(event Collision|EventActorBeginOverlap
  (params (OtherActor :type Actor%20Object%20Reference)))

(event EventTick
  (params (DeltaSeconds :type Float%20%28single-precision%29)))

(fn ConstructionScript
  (Audio|Components|Audio|SetSound (Variables|Default|GetAudio) (Variables|Default|GetMusic)))